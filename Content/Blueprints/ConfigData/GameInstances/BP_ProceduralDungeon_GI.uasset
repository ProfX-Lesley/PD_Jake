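; Game Instance that procedurally builds a dungeon from a seeded random stream, with a random seed when zero is given.
; From a starter room, it spawns extension rooms at random endpoint arrows, destroying overlapping ones and retrying on a timer-driven loop.
; Afterwards, overlapping check boxes filter out joined endpoints, the rest get caps, and an exit spawns at a random extension room.
; In main-menu mode, it builds slowly, then clears and regenerates endlessly.
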(event `/Game/Blueprints/Interfaces/BPI_ProceduralDungeon.InitializeDungeon_IF`
  (`self.VariablesReset`)
  (`self.ProcesSeedInput`)
  (`self.PrintExtensions`)
  (if (`self.IsMainMenu?_GI`)
    (bind _output_get (set `self.BuildDelay` 1.0))
    (`self.GenerateStarterRoom`)
    (`KismetSystemLibrary.Delay` _output_get)
    (`self.GenerateExtensionRooms`)
    (else
      (set `self.BuildDelay` 0.01)
      (`self.GenerateStarterRoom`)
      (`self.GenerateExtensionRooms`))))

(event `NavMeshSetup`
  (bind _returnvalue (`GameplayStatics.GetActorOfClass` "/Script/NavigationSystem.NavMeshBoundsVolume"))
  (set `self.NavMeshRef` _returnvalue)
  (bind _outactors (`GameplayStatics.GetAllActorsOfClassWithTag` "/Game/Blueprints/Actors/DungeonRooms/BP_Room_Master.BP_Room_Master_C" "DungeonRoom"))
  (set `self.AllRooms` _outactors))

(fn `ClearCurrentDungeon`
  (set `self.LoadingSeed` 0)
  (`KismetArrayLibrary.Array_Clear` (`self.CurrentOverlappedComponents`))
  (`self.VariablesReset`)
  (bind _outactors (`GameplayStatics.GetAllActorsOfClass` "/Game/Blueprints/Actors/DungeonRooms/BP_Room_Master.BP_Room_Master_C")) ; Gets all dungeon rooms
  (for _array_element _outactors
    (`Actor.K2_DestroyActor` _array_element) ; Destroy Room
  )
  (bind _outactors_2 (`GameplayStatics.GetAllActorsOfClass` "/Game/Blueprints/Actors/DungeonRooms/BP_RoomCap.BP_RoomCap_C"))
  (for _array_element_2 _outactors_2
    (`Actor.K2_DestroyActor` _array_element_2))
  (`KismetSystemLibrary.CollectGarbage`))

(fn `GenerateExtensionRooms`
  (if (> (`self.Extensions`) 0) :!label _label
    (bind _chosenendpoint (`self.RandomEndpointSelect` (`self.AllEndPoints`)))
    (bind (_chosenextensionclass _chosenextensionclassindex _endpointtransform) (`self.EndPointCheck` _chosenendpoint)
      (:`ValidEndPoint`
        (bind _returnvalue (`|SpawnActorFromClass` _chosenextensionclass _endpointtransform "Undefined" "MultiplyWithRoot" null null))
        (`self.RoomOverlapCheck` _returnvalue
          (:`GoodRoom`
            (`self.SetUpRoom`)
            (`KismetSystemLibrary.K2_SetTimer` null "GenerateExtensionRooms" (`self.BuildDelay`)))
          (:`BadRoom`
            (`Actor.K2_DestroyActor` (`self.CurrentRoom`))
            (goto _label))))
      (:`InvalidEndPoint`
        (`self.ClearCurrentDungeon`) ; FAILSAFE: Clears the current Dungeon
        (goto _label)))
    (elif (`self.IsMainMenu?_GI`)
      (`self.ClearCurrentDungeon`)
      (`self.InitializeDungeon_IF`)
      (else
        (`KismetSystemLibrary.PrintString` "ExtensionsComplete")
        (`self.GenerateEndCheckBoxes`)
        (`self.ProcessValidEndPoints`)
        (`self.GenerateRoomCaps`)
        (`self.CleanUpEndCheckBoxes`)
        (`self.GenerateExit`)))))

(fn `GenerateStarterRoom`
  (bind _returnvalue (`|SpawnActorFromClass` (`self.RandomizeStarterRoom`) (`self.StartRoomSpawnPoint`) "Undefined" "MultiplyWithRoot" null null)) ; Spawns in the starting room.
  (set `self.AllEndPoints` (`self.AllEndPoints`))
  (`KismetArrayLibrary.Array_Append` (`self.AllEndPoints`) (`SceneComponent.GetChildrenComponents` (`/Game/Blueprints/Actors/DungeonRooms/BP_Room_Master.EndPoints_Grp` _returnvalue) false))
  (return))

(fn `ProcesSeedInput`
  (bind _loadingseed (`self.LoadingSeed`))
  (bind _seedstream (`self.SeedStream`))
  (bind _seedstream_initialseed (`KismetMathLibrary.BreakRandomStream` (`self.SeedStream`)))
  (if (== _loadingseed 0)
    (`KismetMathLibrary.SeedRandomStream` _seedstream) ; Similar to a variable setter. \nSets seed to random value.
    (set `self.LoadingSeed` _seedstream_initialseed) ; Used as a referance of the seed
    (else
      (`KismetMathLibrary.SetRandomStreamSeed` _seedstream _loadingseed) ; Looks at users ranodm inputed number\nthen sets that number as the seed
    )))

(fn `RandomizeStarterRoom`
  (returns (Output :type "/Game/Blueprints/Actors/DungeonRooms/BP_Room_Master Class Reference"))
  (bind _startroomclasses (`self.StartRoomClasses`))
  (return (`|GetArrayItem` _startroomclasses (`KismetMathLibrary.RandomIntegerInRangeFromStream` (`self.SeedStream`) 0 (- (`KismetArrayLibrary.Array_Length` _startroomclasses) 1)))))

(fn `VariablesReset`
  (`KismetArrayLibrary.Array_Clear` (`self.AllEndPoints`))
  (set `self.Extensions` (- (`self.TotalRooms`) 1))
  (set `self.CurrentRoom` null)
  (set `self.StartRoomSpawnPoint` (struct)))